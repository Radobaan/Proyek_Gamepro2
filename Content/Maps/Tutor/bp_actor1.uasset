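; Tutorial-map actor that displays a configurable 3D text message, revealed when the player or another object touches its trigger box.
; On BeginPlay it applies the Text, initial Visibility and a single ColorMaterial to all faces of the Text3D component.
; A Box overlap or hit makes the text visible, with no filter on the other actor and no logic to hide it again.
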(event `self.ReceiveBeginPlay`
  (bind _text3d (`self.Text3D`))
  (bind _text3d_2 (`self.Text3D`))
  (bind _colormaterial (`self.ColorMaterial`))
  (`SceneComponent.SetVisibility` _text3d (`self.Visibility?`) false)
  (`Text3DComponent.SetText` _text3d (`self.Text`))
  (`Text3DComponent.SetFrontMaterial` _text3d_2 _colormaterial)
  (`Text3DComponent.SetBackMaterial` _text3d_2 _colormaterial)
  (`Text3DComponent.SetBevelMaterial` _text3d_2 _colormaterial)
  (`Text3DComponent.SetExtrudeMaterial` _text3d_2 _colormaterial))

(event `self.Box.OnComponentBeginOverlap`
  (params (OverlappedComponent :type "PrimitiveComponent Object Reference") (OtherActor :type "Actor Object Reference") (OtherComp :type "PrimitiveComponent Object Reference") (OtherBodyIndex :type Integer) (bFromSweep :type Boolean) (SweepResult :type "HitResult Structure (by ref)"))
  (`SceneComponent.SetVisibility` (`self.Text3D`) true false))

(event `self.Box.OnComponentHit`
  (params (HitComponent :type "PrimitiveComponent Object Reference") (OtherActor :type "Actor Object Reference") (OtherComp :type "PrimitiveComponent Object Reference") (NormalImpulse :type "Vector Structure") (Hit :type "HitResult Structure (by ref)"))
  (`SceneComponent.SetVisibility` (`self.Text3D`) true false))

(fn `UserConstructionScript`)