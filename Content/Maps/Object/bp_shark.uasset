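; Shark hazard Blueprint that patrols back and forth and kills the third-person character on contact.
; A timeline starts at BeginPlay and drives the skeletal mesh's relative location.
; A 3-second delay on the timeline update toggles a loop flag, flipping the mesh's yaw and switching between play and reverse.
; Overlapping the box ragdolls the character, then destroys it two seconds later.
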(event `self.ReceiveBeginPlay`
  (bind (_direction _moving) (`Timeline|Moving` :!label _label)
    (:`Update`
      (`SceneComponent.K2_SetRelativeLocation` (`self.SkeletalMesh`) _moving false false)
      (`KismetSystemLibrary.Delay` 3.0)
      (if (`self.isLooped`)
        (set `self.isLooped` false)
        (`SceneComponent.K2_SetRelativeRotation` (`self.SkeletalMesh`) (struct :`Yaw` 90.0) false false)
        (goto _label :!via `Reverse`)
        (else
          (`SceneComponent.K2_SetRelativeRotation` (`self.SkeletalMesh`) (struct :`Yaw` -90.0) false false)
          (set `self.isLooped` true)
          (goto _label))))))

(event `self.Box.OnComponentBeginOverlap`
  (params (OverlappedComponent :type "PrimitiveComponent Object Reference") (OtherActor :type "Actor Object Reference") (OtherComp :type "PrimitiveComponent Object Reference") (OtherBodyIndex :type Integer) (bFromSweep :type Boolean) (SweepResult :type "HitResult Structure (by ref)"))
  (bind _asthird_person_character (cast `/Game/Manny/ThirdPersonBP/Blueprints/ThirdPersonCharacter` OtherActor))
  (`/Game/Manny/ThirdPersonBP/Blueprints/ThirdPersonCharacter.Ragdoll` _asthird_person_character)
  (`KismetSystemLibrary.Delay` 2.0)
  (`self.K2_DestroyActor` _asthird_person_character))

(fn `UserConstructionScript`)