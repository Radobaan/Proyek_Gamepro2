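; ButtonBP is an interactable button that opens its matching doors for a timed window.
; Interact adds a WB_Countdown widget, starts a two-minute timer on ThirdPersonGameMode and opens every DoorBP whose DoorVal equals ButtonValue.
; Tick polls the game mode and, whenever the timer is not running, searches all DoorBP actors each frame and calls CloseDoor on the matching ones.
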(event `self.ReceiveTick`
  (params (DeltaSeconds :type "Float (single-precision)"))
  (bind _asthird_person_game_mode (cast `/Game/Manny/ThirdPersonBP/Blueprints/ThirdPersonGameMode` (`GameplayStatics.GetGameMode`)))
  (if (not (`/Game/Manny/ThirdPersonBP/Blueprints/ThirdPersonGameMode.TimerStart?` _asthird_person_game_mode))
    (bind _outactors (`GameplayStatics.GetAllActorsOfClass` "/Game/Maps/Object/DoorBP.DoorBP_C"))
    (for _array_element _outactors
      (if (== (`/Game/Maps/Object/DoorBP.DoorVal` _array_element) (`self.ButtonValue`))
        (`/Game/Maps/Object/DoorBP.CloseDoor` _array_element)))))

(event `/Game/Manny/Interface/InteractionInterface.Interact`
  (params (Player :type "Character Object Reference"))
  (bind _returnvalue (`|CreateWidget` "/Game/Manny/Timer/WB_Countdown.WB_Countdown_C"))
  (`UserWidget.AddToViewport` _returnvalue 0)
  (bind _asthird_person_game_mode (cast `/Game/Manny/ThirdPersonBP/Blueprints/ThirdPersonGameMode` (`GameplayStatics.GetGameMode`)))
  (set `/Game/Manny/ThirdPersonBP/Blueprints/ThirdPersonGameMode.TimerStart?` true _asthird_person_game_mode)
  (set `/Game/Manny/ThirdPersonBP/Blueprints/ThirdPersonGameMode.Second` 120 _asthird_person_game_mode)
  (bind _outactors (`GameplayStatics.GetAllActorsOfClass` "/Game/Maps/Object/DoorBP.DoorBP_C"))
  (for _array_element _outactors
    (if (== (`/Game/Maps/Object/DoorBP.DoorVal` _array_element) (`self.ButtonValue`))
      (`/Game/Maps/Object/DoorBP.OpenDoor` _array_element))))

(fn `UserConstructionScript`)